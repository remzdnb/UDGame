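; Player controller Blueprint that relays camera input to the RDBCameraManager.
; Movement and look axis events cast the PlayerCameraManager to RDBCameraManager and pass the axis values to its matching functions.
; The ToggleFreeLook action works as a hold, sending true on press and false on release.
; It keeps no logic of its own, and input does nothing if the cast fails.
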(event Input|ActionEvents|InputActionToggleFreeLook
  (params (Key :type Key%20Structure :default "None"))
  (:Pressed
    (bind _asrdbcamera_manager (Utilities|Casting|CastToRDBCameraManager (Variables|Default|GetPlayerCameraManager)))
    (Class|RDBCameraManager|ToggleFreeLook _asrdbcamera_manager true))
  (:Released
    (bind _asrdbcamera_manager_2 (Utilities|Casting|CastToRDBCameraManager (Variables|Default|GetPlayerCameraManager)))
    (Class|RDBCameraManager|ToggleFreeLook _asrdbcamera_manager_2 false)))

(event Input|AxisEvents|InputAxisMoveForward
  (params (AxisValue :type Float%20%28single-precision%29))
  (bind _asrdbcamera_manager (Utilities|Casting|CastToRDBCameraManager (Variables|Default|GetPlayerCameraManager)))
  (Class|RDBCameraManager|MoveForward _asrdbcamera_manager AxisValue))

(event Input|AxisEvents|InputAxisMoveRight
  (params (AxisValue :type Float%20%28single-precision%29))
  (bind _asrdbcamera_manager (Utilities|Casting|CastToRDBCameraManager (Variables|Default|GetPlayerCameraManager)))
  (Class|RDBCameraManager|MoveRight _asrdbcamera_manager AxisValue))

(event Input|AxisEvents|InputAxisLookRight
  (params (AxisValue :type Float%20%28single-precision%29))
  (bind _asrdbcamera_manager (Utilities|Casting|CastToRDBCameraManager (Variables|Default|GetPlayerCameraManager)))
  (Class|RDBCameraManager|LookRight _asrdbcamera_manager AxisValue))

(event Input|AxisEvents|InputAxisLookUp
  (params (AxisValue :type Float%20%28single-precision%29))
  (bind _asrdbcamera_manager (Utilities|Casting|CastToRDBCameraManager (Variables|Default|GetPlayerCameraManager)))
  (Class|RDBCameraManager|LookUp _asrdbcamera_manager AxisValue))

(fn ConstructionScript)